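; Interactive shower actor that starts its Water component when switched on with the E key.
; Any overlap with Box enables player input on the actor, and ending the overlap disables it.
; Each E press toggles ShowerOn and plays an attenuated shower sound at the actor's location.
; Water begins paused; Tick unpauses it while ShowerOn is true, but nothing pauses it again when switched off.
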(event OnComponentBeginOverlap(Box)
  (params (OverlappedComponent :type Primitive%20Component%20Object%20Reference) (OtherActor :type Actor%20Object%20Reference) (OtherComp :type Primitive%20Component%20Object%20Reference) (OtherBodyIndex :type Integer) (bFromSweep :type Boolean) (SweepResult :type Hit%20Result%20Structure%20%28by%20ref%29))
  (Input|EnableInput (Game|GetPlayerController 0)))

(event OnComponentEndOverlap(Box)
  (params (OverlappedComponent :type Primitive%20Component%20Object%20Reference) (OtherActor :type Actor%20Object%20Reference) (OtherComp :type Primitive%20Component%20Object%20Reference) (OtherBodyIndex :type Integer))
  (Input|DisableInput (Game|GetPlayerController 0)))

(event EventBeginPlay
  (Class|NiagaraComponent|SetPaused (Variables|Default|GetWater) true))

(event Collision|EventActorBeginOverlap
  (params (OtherActor :type Actor%20Object%20Reference)))

(event EventTick
  (params (DeltaSeconds :type Float%20%28single-precision%29))
  (if (Variables|Default|GetShowerOn)
    (Class|NiagaraComponent|SetPaused (Variables|Default|GetWater) false)))

(event Input|KeyboardEvents|E
  (params (Key :type Key%20Structure :default "None"))
  (:Pressed
    (Variables|Default|SetShowerOn (not (Variables|Default|GetShowerOn)))
    (Audio|PlaySoundatLocation "/Game/StarterContent/Audio/Downloads/shower.shower" (Transformation|GetActorLocation) "0, 0, 0" 1.0 1.0 0.0 "/Game/StarterContent/Audio/Downloads/shower_attenuation.shower_attenuation" 0 0)))

(fn ConstructionScript)