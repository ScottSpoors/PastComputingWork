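; Elevator door actor that endlessly opens and closes by moving vertically between its starting height and a point 300 units above.
; BeginPlay stores both endpoints, and Tick counts down a frame-based delay before shifting Z by Speed and playing the door sound on every moving frame.
; An exact float match with either endpoint resets the delay and reverses Speed, so motion depends on frame rate and step size.
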(event EventBeginPlay
  ;[1 1 1] Initialises start and end point variables
  (bind _output_get (Variables|Default|SetOrigin (.Z (Math|Vector|BreakVector (Transformation|GetActorLocation)))))
  (Variables|Default|SetEndPoint (+ _output_get 3e+02)))

(event Collision|EventActorBeginOverlap
  (params (OtherActor :type Actor%20Object%20Reference)))

(event EventTick
  (params (DeltaSeconds :type Float%20%28single-precision%29))
  (bind _returnvalue (Transformation|GetActorLocation))
  (bind (_x _y _z) (Math|Vector|BreakVector _returnvalue))
  ;[1 1 1] Results in door constantly opening and closing
  (Variables|Default|SetDelay (- (Variables|Default|GetDelay) 1))
  (if (<= (Variables|Default|GetDelay) 0)
    (Audio|PlaySoundatLocation "/Game/StarterContent/Audio/Downloads/elevator-door.elevator-door" (Transformation|GetActorLocation) "0, 0, 0" 1.0 1.0 0.0 "/Game/StarterContent/Audio/Downloads/elevator-door_attenuation.elevator-door_attenuation" 0 0)
    (Transformation|SetActorLocation (Math|Vector|MakeVector _x _y (+ (stale _output_get) _z)) false false)
    (if (or (== (.Z (Math|Vector|BreakVector (Transformation|GetActorLocation))) (Variables|Default|GetEndPoint)) (== (.Z (Math|Vector|BreakVector (Transformation|GetActorLocation))) (Variables|Default|GetOrigin)))
      (Variables|Default|SetDelay (Variables|Default|GetDoorDelay))
      (bind _output_get (Variables|Default|SetSpeed (* (Variables|Default|GetSpeed) -1.0))))))

(fn ConstructionScript)