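; Bomb placement spot where a player carrying a bomb presses E to plant it, causing a timed explosion.
; The box overlap toggles input and tracks whether the player is in range; planting reveals the bomb mesh and consumes the player's bomb.
; Tick runs a Delay while the bomb is placed, then hides it, fires the particle effect with sound, and subtracts health from a player still in range.
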(event OnComponentBeginOverlap(Box)
  (params (OverlappedComponent :type Primitive%20Component%20Object%20Reference) (OtherActor :type Actor%20Object%20Reference) (OtherComp :type Primitive%20Component%20Object%20Reference) (OtherBodyIndex :type Integer) (bFromSweep :type Boolean) (SweepResult :type Hit%20Result%20Structure%20%28by%20ref%29))
  (Input|EnableInput (Game|GetPlayerController 0))
  (Variables|Default|SetPlayerInRange true))

(event OnComponentEndOverlap(Box)
  (params (OverlappedComponent :type Primitive%20Component%20Object%20Reference) (OtherActor :type Actor%20Object%20Reference) (OtherComp :type Primitive%20Component%20Object%20Reference) (OtherBodyIndex :type Integer))
  (Input|DisableInput (Game|GetPlayerController 0))
  (Variables|Default|SetPlayerInRange false))

(event OnComponentActivated(P_Explosion)
  (params (Component :type Actor%20Component%20Object%20Reference) (bReset :type Boolean))
  (Audio|PlaySoundatLocation "/Game/StarterContent/Audio/Explosion_Cue.Explosion_Cue" (Transformation|GetWorldLocation (Variables|Default|GetP_Explosion)) "0, 0, 0" 1.0 1.0 0.0 0 0 0))

(event EventBeginPlay
  (Rendering|SetVisibility (Variables|Default|GetBomb) false false)
  (Variables|Default|SetBombPlaced false)
  (Components|Activation|Deactivate (Variables|Default|GetP_Explosion)))

(event Collision|EventActorBeginOverlap
  (params (OtherActor :type Actor%20Object%20Reference)))

(event EventTick
  (params (DeltaSeconds :type Float%20%28single-precision%29))
  (if (Variables|Default|GetBombPlaced)
    (Utilities|FlowControl|Delay 5.0)
    (Components|Activation|Activate (Variables|Default|GetP_Explosion) true)
    (Variables|Default|SetIsExploding true)
    (Rendering|SetVisibility (Variables|Default|GetBomb) false false)
    (Variables|Default|SetIsExploding false)
    (Variables|Default|SetBombPlaced false)
    (if (Variables|Default|GetPlayerInRange)
      (bind _asthird_person_character (Utilities|Casting|CastToThirdPersonCharacter (stale OnComponentBeginOverlap(Box) OtherActor)))
      (Variables|/Game/ThirdPersonBP/Blueprints/ThirdPersonCharacter.ThirdPersonCharacter_C|SetPlayerHealth _asthird_person_character (- (Variables|/Game/ThirdPersonBP/Blueprints/ThirdPersonCharacter.ThirdPersonCharacter_C|GetPlayerHealth _asthird_person_character) 3.0))
      (Development|PrintText "Player took 3 damage"))))

(event Input|KeyboardEvents|E
  (params (Key :type Key%20Structure :default "None"))
  (:Pressed
    (bind _asthird_person_character (Utilities|Casting|CastToThirdPersonCharacter (stale OnComponentBeginOverlap(Box) OtherActor)))
    (if (Variables|/Game/ThirdPersonBP/Blueprints/ThirdPersonCharacter.ThirdPersonCharacter_C|GetHasBomb _asthird_person_character)
      (Rendering|SetVisibility (Variables|Default|GetBomb) true false)
      (Variables|Default|SetBombPlaced true)
      (Variables|/Game/ThirdPersonBP/Blueprints/ThirdPersonCharacter.ThirdPersonCharacter_C|SetHasBomb _asthird_person_character false))))

(fn ConstructionScript)