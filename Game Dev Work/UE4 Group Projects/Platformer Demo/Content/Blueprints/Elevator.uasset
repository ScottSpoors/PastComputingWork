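; Elevator actor that carries the player upward to a top point when they press E while standing on it.
; A Box overlap toggles player input and the OnElevator flag, and E sets Move.
; Tick raises the actor by MovementRate per frame without delta-time scaling, then stops and disables input at TopPoint.
; The movement sound is gated by IsPlaying, which this graph never sets.
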(event OnComponentBeginOverlap(Box)
  (params (OverlappedComponent :type Primitive%20Component%20Object%20Reference) (OtherActor :type Actor%20Object%20Reference) (OtherComp :type Primitive%20Component%20Object%20Reference) (OtherBodyIndex :type Integer) (bFromSweep :type Boolean) (SweepResult :type Hit%20Result%20Structure%20%28by%20ref%29))
  ;[1 1 1] Controls movement and sound output of elevator based on user location and input
  (Input|EnableInput (Game|GetPlayerController 0))
  (Variables|Default|SetOnElevator true))

(event OnComponentEndOverlap(Box)
  (params (OverlappedComponent :type Primitive%20Component%20Object%20Reference) (OtherActor :type Actor%20Object%20Reference) (OtherComp :type Primitive%20Component%20Object%20Reference) (OtherBodyIndex :type Integer))
  ;[1 1 1] Controls movement and sound output of elevator based on user location and input
  (Input|DisableInput (Game|GetPlayerController 0))
  (Variables|Default|SetOnElevator false))

(event EventTick
  (params (DeltaSeconds :type Float%20%28single-precision%29))
  (bind _returnvalue (Transformation|GetActorLocation))
  (bind (_x _y _z) (Math|Vector|BreakVector _returnvalue))
  ;[1 1 1] Controls movement and sound output of elevator based on user location and input
  (if (and (Variables|Default|GetMove) (Variables|Default|GetOnElevator))
    (if (Variables|Default|GetisPlaying)
      _
      (else
        (Audio|PlaySoundatLocation "/Game/StarterContent/Audio/Downloads/elevator-move.elevator-move" (Transformation|GetActorLocation) "0, 0, 0" 1.0 1.0 0.0 "/Game/StarterContent/Audio/Downloads/elevator-move_attenuation.elevator-move_attenuation" 0 0)))
    (Transformation|SetActorLocation (Math|Vector|MakeVector _x _y (+ _z (Variables|Default|GetMovementRate))) false false)
    (if (>= _z (Variables|Default|GetTopPoint))
      (Variables|Default|SetMove false)
      (Input|DisableInput (Game|GetPlayerController 0)))))

(event Input|KeyboardEvents|E
  (params (Key :type Key%20Structure :default "None"))
  ;[1 1 1] Controls movement and sound output of elevator based on user location and input
  (:Pressed
    (Variables|Default|SetMove true)))

(fn ConstructionScript)