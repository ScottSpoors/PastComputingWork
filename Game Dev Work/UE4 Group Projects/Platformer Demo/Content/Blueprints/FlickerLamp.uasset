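; FlickerLamp is a lamp Blueprint whose spot light blinks off at random intervals while its Flicker flag is set.
; Tick drives the loop through latent Delays, waiting a random whole number of seconds bounded by FlickerRate before briefly hiding the SpotLight.
; When the light turns back on, a flicker sound plays at the actor's location.
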(event EventBeginPlay)

(event Collision|EventActorBeginOverlap
  (params (OtherActor :type Actor%20Object%20Reference)))

(event EventTick
  (params (DeltaSeconds :type Float%20%28single-precision%29))
  (if (Variables|Default|GetFlicker)
    (Utilities|FlowControl|Delay (Math|Conversions|ToFloat(Integer) (Math|Random|RandomInteger (Variables|Default|GetFlickerRate))))
    (Rendering|SetVisibility (Variables|Default|GetSpotLight) false false)
    (Utilities|FlowControl|Delay 0.2)
    (Rendering|SetVisibility (Variables|Default|GetSpotLight) true false)
    (Audio|PlaySoundatLocation "/Game/StarterContent/Audio/Downloads/flicker.flicker" (Transformation|GetActorLocation) "0, 0, 0" 1.0 1.0 0.0 "/Game/StarterContent/Audio/Downloads/flicker_attenuation.flicker_attenuation" 0 0)))

(fn ConstructionScript)